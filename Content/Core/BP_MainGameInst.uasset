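; BP_MainGameInst, apparently the main game instance, wraps a PakDownloader for fetching game content as pak chunks.
; InitPakDownloader creates the downloader if needed, initializes it with a hard-coded internal-test Windows build config, and broadcasts the inverted result as whether new paks exist.
; It relays download-completion events with chunk ID and success through its own dispatcher.
; Helper functions start downloads by chunk ID or translate chunk status into Chinese text.
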(event `InitPakDownloader`
  (`self.PakDownloaderInst`
    (:`then`
      _)
    (:`else`
      (bind _returnvalue (`|GenericCreateObject` "/Script/PakUseCase.PakDownloader"))
      (bind _output_get (set `self.PakDownloaderInst` _returnvalue))))
  (bind _returnvalue_2 (`PakDownloader.InitDownloader` _output_get "InternalTest" "Chapt2nd" "Windows"))
  (`self.IsHaveNewPaks` (not _returnvalue_2))
  (add `PakDownloader.PakDownloadEvt` _output_get (delegate `PakDownloadEvt_Event`)))

(event `PakDownloadEvt_Event`
  (params (ChunkID :type Integer) (IsSuccess :type Boolean))
  (`self.PakDownloadEvtFired` ChunkID IsSuccess))

(fn `CheckChunkByID`
  (params (ID :type Integer))
  (returns (RslTxt :type String))
  (bind _pakdownloaderinst (`self.PakDownloaderInst`)
    (:`then`
      (bind _returnvalue (`PakDownloader.CheckChunkById` _pakdownloaderinst ID))
      (switch `int` _returnvalue
        (:`Default`
          (return "未知..."))
        (:`0`
          (return "已经挂载"))
        (:`1`
          (return "本地有缓存但未挂载"))
        (:`2`
          (return "正在下载"))
        (:`3`
          (return "本地部分缓存"))
        (:`4`
          (return "本地无缓存"))))
    (:`else`)))

(fn `DownloadPakByID`
  (params (ID :type Integer))
  (bind _pakdownloaderinst (`self.PakDownloaderInst`)
    (:`then`
      (`PakDownloader.DownloadChunkById` _pakdownloaderinst ID))
    (:`else`)))